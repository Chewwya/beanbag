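; Moving platform that carries its static mesh along a spline, started and stopped by a linked pressure switch.
; A flag decides whether pressing starts movement and releasing stops it, or the reverse.
; A timeline, rate-scaled by duration, maps progress to spline distance for position and optional rotation, and ping-pongs at each end.
; The construction script applies the platform material.
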(event `self.ReceiveBeginPlay`
  (`|ExecutionSequence`
    (:`then_0`
      (add `/Game/Blueprints/PressureSwitch.SwitchPressed` (`self.ButtonReference`) (delegate `SwitchPressed`)))
    (:`then_1`
      (add `/Game/Blueprints/PressureSwitch.SwitchReleased` (`self.ButtonReference`) (delegate `SwitchReleased`)))))

(event `SwitchPressed`
  (params (PressureSwitch :type "/Game/Blueprints/PressureSwitch Object Reference"))
  (bind _spline (`self.Spline`))
  (bind _staticmesh (`self.StaticMesh`))
  (if (== PressureSwitch (`self.ButtonReference`))
    (if (`self.ButtonActivatesMovement?`)
      (`TimelineComponent.SetPlayRate` (`self.MovePlatformTimeline`) (/ 1.0 (`self.Duration`)) :!label _label)
      (bind (_direction _traveldistance) (`Timeline|MovePlatformTimeline` :!label _label_2)
        (:`Update`
          (bind _returnvalue (* _traveldistance (`SplineComponent.GetSplineLength` _spline)))
          (`SceneComponent.K2_SetWorldLocation` _staticmesh (`SplineComponent.GetLocationAtDistanceAlongSpline` _spline _returnvalue "World") false false)
          (if (`self.ModifyRotation?`)
            (`SceneComponent.K2_SetRelativeRotation` _staticmesh (`SplineComponent.GetRotationAtDistanceAlongSpline` _spline _returnvalue "Local") false false)))
        (:`Finished`
          (switch `ETimelineDirection` _direction
            (:`Forward`
              (goto _label_2 :!via `Reverse`))
            (:`Backward`
              (goto _label_2)))))
      (else
        (goto _label_2 :!via `Stop`)))))

(event `SwitchReleased`
  (params (PressureSwitch :type "/Game/Blueprints/PressureSwitch Object Reference"))
  (if (== PressureSwitch (`self.ButtonReference`))
    (if (`self.ButtonActivatesMovement?`)
      (goto _label_2 :!via `Stop`)
      (else
        (goto _label)))))

(fn `UserConstructionScript`
  (`PrimitiveComponent.SetMaterial` (`self.StaticMesh`) 0 (`self.PlatformMaterial`)))