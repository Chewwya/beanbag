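; Pressure switch actor that reacts when a BeanbagCharacter or TestBox stands on it.
; Box overlaps adjust an occupant count, set the pressed flag and lower or raise the button mesh.
; Tick watches the count and uses two cross-resetting DoOnce nodes to fire SwitchPressed and SwitchReleased once per change.
; Any single exit raises the button and clears the flag, even with other occupants remaining.
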(event `self.Box.OnComponentBeginOverlap`
  (params (OverlappedComponent :type "PrimitiveComponent Object Reference") (OtherActor :type "Actor Object Reference") (OtherComp :type "PrimitiveComponent Object Reference") (OtherBodyIndex :type Integer) (bFromSweep :type Boolean) (SweepResult :type "HitResult Structure (by ref)"))
  (cast `/Game/Blueprints/BeanbagCharacter` OtherActor
    (:`then`
      _)
    (:`CastFailed`
      (cast `/Game/Blueprints/TestBox` OtherActor)))
  (`/Engine/EditorBlueprintResources/StandardMacros.IncrementInt` (`self.NumberOfObjectsOnSwitch`)
    (:`  `
      (set `self.IsButtonPressed` true)
      (`SceneComponent.K2_SetRelativeLocation` (`self.Button`) (0.0 0.0 -10.0) false false))))

(event `self.Box.OnComponentEndOverlap`
  (params (OverlappedComponent :type "PrimitiveComponent Object Reference") (OtherActor :type "Actor Object Reference") (OtherComp :type "PrimitiveComponent Object Reference") (OtherBodyIndex :type Integer))
  (cast `/Game/Blueprints/BeanbagCharacter` OtherActor
    (:`then`
      _)
    (:`CastFailed`
      (cast `/Game/Blueprints/TestBox` OtherActor)))
  (`/Engine/EditorBlueprintResources/StandardMacros.DecrementInt` (`self.NumberOfObjectsOnSwitch`)
    (:`  `
      (set `self.IsButtonPressed` false)
      (`SceneComponent.K2_SetRelativeLocation` (`self.Button`) (0.0 0.0 -5.0) false false))))

(event `self.ReceiveTick`
  (params (DeltaSeconds :type "Float (single-precision)"))
  (if (> (`self.NumberOfObjectsOnSwitch`) 0)
    (`/Engine/EditorBlueprintResources/StandardMacros.DoOnce` false :!label _label
      (:`Completed`
        (`self.SwitchPressed` self)
        (goto _label_2 :!via `Reset`)))
    (else
      (`/Engine/EditorBlueprintResources/StandardMacros.DoOnce` false :!label _label_2
        (:`Completed`
          (`self.SwitchReleased` self)
          (goto _label :!via `Reset`))))))

(fn `UserConstructionScript`)